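; BP_ItemSpawner is an actor that periodically spawns a random item at its own transform.
; On BeginPlay it starts a looping timer at SpawnRate that calls SpawnRandomItem by name.
; Each call spawns a BP_BaseItem, then passes a random row name from ItemDataTable to InitializeItem through the BPI_Initializable interface, so the item is configured only after spawning finishes.
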(event `self.ReceiveBeginPlay`
  (`KismetSystemLibrary.K2_SetTimer` self "SpawnRandomItem" (`self.SpawnRate`) true))

(fn `SpawnRandomItem`
  (bind _returnvalue (`SceneComponent.K2_GetComponentToWorld` (`self.K2_GetRootComponent`)))
  (bind _outrownames (`DataTableFunctionLibrary.GetDataTableRowNames` (`self.ItemDataTable`)))
  (bind _returnvalue_2 (`GameplayStatics.BeginDeferredActorSpawnFromClass` "/Game/FirstPerson/Blueprints/BP_BaseItem.BP_BaseItem_C" _returnvalue "Undefined" null))
  (bind _returnvalue_3 (`GameplayStatics.FinishSpawningActor` _returnvalue_2 _returnvalue))
  (bind _asbpi_initializable (cast `/Game/BPI_Initializable` _returnvalue_3))
  (`/Game/BPI_Initializable.InitializeItem` _asbpi_initializable (`KismetArrayLibrary.Array_Get` _outrownames (`KismetMathLibrary.RandomIntegerInRange` 0 (`KismetArrayLibrary.Array_LastIndex` _outrownames))))
  (return))

(fn `UserConstructionScript`)